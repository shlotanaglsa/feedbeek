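; BP_CellsObject is a data container that holds an array of cell items alongside a Dimensions value.
; Getter functions expose the dimensions and the item array, while SetItem writes an item at a given index.
; RemoveItemAtIndex performs the same overwrite with the item passed in, so it replaces the slot's contents rather than deleting the array element.
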(fn `Get_Dimensions`
  (returns (Dimensions :type "IntPoint Structure"))
  (return (`self.Dimensions`)))

(fn `Get_Items`
  (returns (Items :type "Array of /Game/InventorySystem_0_4/Blueprints/Structures/F_Item Structure"))
  (return (`self.Array_Items`)))

(fn `RemoveItemAtIndex`
  (params (Index :type Integer) (Item :type "/Game/InventorySystem_0_4/Blueprints/Structures/F_Item Structure (by ref)"))
  (`KismetArrayLibrary.Array_Set` (`self.Array_Items`) Index Item))

(fn `Set_Item`
  (params (Index :type Integer) (Item :type "/Game/InventorySystem_0_4/Blueprints/Structures/F_Item Structure (by ref)"))
  (`KismetArrayLibrary.Array_Set` (`self.Array_Items`) Index Item))