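; BP_ItemObject is the object representation of an inventory item, holding its item struct, table data, dimensions, action type and rotation state.
; Setup writes a self-reference into the Item struct, then loads its data table row to cache ItemData, Dimension and ActionType.
; SetRotated toggles rotation by swapping X and Y, skipping square items.
; Accessors expose this state and a settable ArrayItemInventory for the item's own inventory.
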(fn `Get_ActionsType`
  (returns (`Action Type` :type "Array of /Game/InventorySystem_0_4/Blueprints/Enumerations/E_ItemActionType Enum"))
  (return (`self.Action Type`)))

(fn `Get_Dimensions`
  (returns (Dimension :type "IntPoint Structure"))
  (return (`self.Dimension`)))

(fn `Get_IsRotated`
  (returns (`IsRotated?` :type Boolean))
  (return (`self.IsRotated?`)))

(fn `Get_Item`
  (returns (Item :type "/Game/InventorySystem_0_4/Blueprints/Structures/F_Item Structure"))
  (return (`self.Item`)))

(fn `Get_ItemData`
  (returns (ItemData :type "/Game/InventorySystem_0_4/Blueprints/Structures/F_ItemData Structure"))
  (return (`self.ItemData`)))

(fn `Get_ItemInventory`
  (returns (ItemInventory :type "Array of /Game/InventorySystem_0_4/Blueprints/Structures/F_ContainerRow Structure"))
  (return (`self.Array_ItemInventory`)))

(fn `Set_Item`
  (params (Item :type "/Game/InventorySystem_0_4/Blueprints/Structures/F_Item Structure"))
  (set `self.Item` Item))

(fn `Set_ItemInventory`
  (params (Array_ItemInventory :type "Array of /Game/InventorySystem_0_4/Blueprints/Structures/F_ContainerRow Structure"))
  (set `self.Array_ItemInventory` Array_ItemInventory))

(fn `Set_Rotated`
  (bind (_dimension_x _dimension_y) (break `IntPoint` (`self.Dimension`)))
  (bind (_dimension_x_2 _dimension_y_2) (break `IntPoint` (`self.Dimension`)))
  (if (not (== _dimension_x _dimension_y))
    (set `self.IsRotated?` (not (`self.IsRotated?`)))
    (set `self.Dimension` (make `IntPoint` _dimension_y_2 _dimension_x_2))))

(fn `Setup`
  (bind _structout (setmembers `/Game/InventorySystem_0_4/Blueprints/Structures/F_Item` :`StructRef` (`self.Item`) :`ItemObject` self))
  (bind _output_get (set `self.Item` _structout))
  (bind (_datatable _rowname) (break `DataTableRowHandle` (`.Item_2_7B2F9D1C44664DE095F72AA76ADB4E1C` (break `/Game/InventorySystem_0_4/Blueprints/Structures/F_Item` _output_get))))
  (bind _returnvalue (`|GetDataTableRow` _datatable _rowname)
    (:`then`
      (bind _output_get_2 (set `self.ItemData` _returnvalue))
      (bind ((`Dimension_17_233C9396487AF68A332368BB1F978C83` _dimension) (`ActionType_46_9D4776BD4CED402074173D909C55FBCD` _actiontype)) (break `/Game/InventorySystem_0_4/Blueprints/Structures/F_ItemData` _output_get_2))
      (set `self.Dimension` _dimension)
      (set `self.Action Type` _actiontype))))