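; World item pickup actor that wraps an item struct in a BP_ItemObject and takes its mesh from item data.
; The item's pickup method selects line trace, overlap collision or auto-grab by destroying unused spheres; auto-grab flies the item to the character via timeline.
; Focus shows a custom-depth highlight and item widget.
; A multicast update refreshes the mesh and launches it with projectile movement, which starts vertical bobbing on a blocking stop.
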(event `self.ReceiveBeginPlay`
  ;[1 1 1 0.5] Begin Play
  ;;[1 1 1 0.5] Update Projectile Movement
  (`MovementComponent.SetUpdatedComponent` (`self.ProjectileMovement`) (`self.StaticMesh`))
  ;;[1 1 1 0.5] Create New Uobject item
  (bind _returnvalue (`|GenericCreateObject` "/Game/InventorySystem_0_4/Blueprints/Objects/BP_ItemObject.BP_ItemObject_C" (`self.Array_Inventory`) (`self.Item`)))
  (`/Game/InventorySystem_0_4/Blueprints/Objects/BP_ItemObject.Setup` _returnvalue)
  (bind _structout (setmembers `/Game/InventorySystem_0_4/Blueprints/Structures/F_Item` :`StructRef` (`self.Item`) :`ItemObject` _returnvalue))
  (set `self.Item` _structout)
  ;[1 1 1 0.5] Setup Item Pickup Method
  (switch `/Game/InventorySystem_0_4/Blueprints/Enumerations/E_ItemPickupMethod` (`self.ItemPickupMethod`)
    (:`NewEnumerator0`
      (`ActorComponent.K2_DestroyComponent` (`self.SphereCollision_AutoGrab`))
      (`ActorComponent.K2_DestroyComponent` (`self.SphereCollision_Pickup`)))
    (:`NewEnumerator1`
      (`ActorComponent.K2_DestroyComponent` (`self.SphereCollision_Pickup`)))
    (:`NewEnumerator2`
      (`ActorComponent.K2_DestroyComponent` (`self.SphereCollision_AutoGrab`)))))

(event `self.ProjectileMovement.OnProjectileStop`
  (params (ImpactResult :type "HitResult Structure (by ref)"))
  ;[1 1 1 0.5] Can Start Animation
  (bind _output_get (set `self.ProjectileMovementIsStop` (`GameplayStatics.BreakHitResult` ImpactResult)))
  (if _output_get
    (`self.Start Animation`)))

(event `Start Animation`
  ;[1 1 1 0.5] Vertical Oscillation (Animation)
  (if (not (`TimelineComponent.IsPlaying` (`self.Vertical Oscillation`)))
    (set `self.CurrentActorLocation` (`self.K2_GetActorLocation`))
    (`KismetSystemLibrary.Delay` 0.2)
    (bind (_direction _alpha) (`Timeline|Vertical Oscillation`)
      (:`Update`
        (`self.K2_SetActorLocation` (`KismetMathLibrary.VLerp` (`self.CurrentActorLocation`) (`KismetMathLibrary.MakeVector` (.x (`self.CurrentActorLocation`)) (.y (`self.CurrentActorLocation`)) (+ (.z (`self.CurrentActorLocation`)) 4.0)) _alpha))))))

(event `/Game/InventorySystem_0_4/Blueprints/Interfaces/BPI_Interaction.Set_FocusInteraction`
  (params (IsFocus :type Boolean))
  ;[1 1 1 0.5] Set Focus Interaction (interface)
  (`self.UpdateVisual` IsFocus))

(event `Update Item (multicast)`
  (params (Item :type "/Game/InventorySystem_0_4/Blueprints/Structures/F_Item Structure"))
  ;[1 1 1 0.5] Update Item (multicast)
  (`self.Update_Item` Item))

(event `self.SphereCollision_Pickup.OnComponentBeginOverlap`
  (params (OverlappedComponent :type "PrimitiveComponent Object Reference") (OtherActor :type "Actor Object Reference") (OtherComp :type "PrimitiveComponent Object Reference") (OtherBodyIndex :type Integer) (bFromSweep :type Boolean) (SweepResult :type "HitResult Structure (by ref)"))
  ;[1 1 1 0.5] SphereCollision Pickup method
  (bind _ascharacter (cast `Character` OtherActor))
  (bind _returnvalue (message `/Game/InventorySystem_0_4/Blueprints/Interfaces/BPI_CH.Get_PlayerController` _ascharacter))
  (message `/Game/InventorySystem_0_4/Blueprints/Interfaces/BI_PC_InventoryComponent.Set_CurrentOverlappedActor` _returnvalue self)
  (`self.UpdateVisual` true))

(event `self.SphereCollision_Pickup.OnComponentEndOverlap`
  (params (OverlappedComponent :type "PrimitiveComponent Object Reference") (OtherActor :type "Actor Object Reference") (OtherComp :type "PrimitiveComponent Object Reference") (OtherBodyIndex :type Integer))
  ;[1 1 1 0.5] SphereCollision Pickup method
  (bind _ascharacter (cast `Character` OtherActor))
  (bind _returnvalue (message `/Game/InventorySystem_0_4/Blueprints/Interfaces/BPI_CH.Get_PlayerController` _ascharacter))
  (message `/Game/InventorySystem_0_4/Blueprints/Interfaces/BI_PC_InventoryComponent.Set_CurrentOverlappedActor` _returnvalue null)
  (`self.UpdateVisual` false))

(event `self.SphereCollision_AutoGrab.OnComponentBeginOverlap`
  (params (OverlappedComponent :type "PrimitiveComponent Object Reference") (OtherActor :type "Actor Object Reference") (OtherComp :type "PrimitiveComponent Object Reference") (OtherBodyIndex :type Integer) (bFromSweep :type Boolean) (SweepResult :type "HitResult Structure (by ref)"))
  ;[1 1 1 0.5] Sphere Collision AutoGrab Method
  (bind _ascharacter (cast `Character` OtherActor))
  (bind _output_get (set `self.CharacterReference` _ascharacter))
  (bind _returnvalue (message `/Game/InventorySystem_0_4/Blueprints/Interfaces/BPI_CH.Get_PlayerController` _output_get))
  (bind _returnvalue_2 (message `/Game/InventorySystem_0_4/Blueprints/Interfaces/BI_PC_InventoryComponent.CanAddItemFromActor` _returnvalue (`self.Item`)))
  (if _returnvalue_2
    (`TimelineComponent.Stop` (`self.Vertical Oscillation`))
    (`KismetSystemLibrary.Delay` 0.06)
    (`TimelineComponent.Play` (`self.Timeline Auto Grab`))))

(event `self.SphereCollision_AutoGrab.OnComponentEndOverlap`
  (params (OverlappedComponent :type "PrimitiveComponent Object Reference") (OtherActor :type "Actor Object Reference") (OtherComp :type "PrimitiveComponent Object Reference") (OtherBodyIndex :type Integer))
  ;[1 1 1 0.5] Sphere Collision AutoGrab Method
  (cast `Character` OtherActor)
  (`self.Start Animation`)
  (`MovementComponent.SetUpdatedComponent` (`self.ProjectileMovement`) (`self.StaticMesh`)))

(fn `Update_Item`
  (params (Item :type "/Game/InventorySystem_0_4/Blueprints/Structures/F_Item Structure"))
  (bind _widget_focusinteraction (`self.Widget_FocusInteraction`))
  ;[1 1 1 0.5] Set Static Mesh
  (bind _itemdata (`/Game/InventorySystem_0_4/Blueprints/Library/BFL_Shortcut.Get_ItemData` Item))
  (`StaticMeshComponent.SetStaticMesh` (`self.StaticMesh`) (`.StaticMesh_20_D34A863A40279183967777A1310ABFB5` (break `/Game/InventorySystem_0_4/Blueprints/Structures/F_ItemData` _itemdata)))
  ;[1 1 1 0.5] Add Velocity
  (`ProjectileMovementComponent.SetVelocityInLocalSpace` (`self.ProjectileMovement`) (500.0 0.0 0.0))
  ;[1 1 1 0.5] Update Item Focus Widget
  (`/Engine/EditorBlueprintResources/StandardMacros.IsValid` _widget_focusinteraction
    (:`Is Valid`
      (if (`Widget.IsVisible` _widget_focusinteraction)
        (`/Game/InventorySystem_0_4/Blueprints/UserInterfaces/Game/Item/WBP_FocusItem.Set_Item` _widget_focusinteraction (`self.Item`))))))

(fn `UpdateVisual`
  (params (`IsFocus?` :type Boolean))
  (bind _widget_focusinteraction (`self.Widget_FocusInteraction`))
  (bind _staticmesh (`self.StaticMesh`))
  (bind _staticmesh_2 (`self.StaticMesh`))
  (if `IsFocus?`
    ;[1 1 1 0.5] Highlight Materials
    (`PrimitiveComponent.SetRenderCustomDepth` _staticmesh_2 true)
    (`PrimitiveComponent.SetCustomDepthStencilValue` _staticmesh_2 2)
    ;[1 1 1 0.5] Focus Widget Visibility
    (`SceneComponent.SetHiddenInGame` (`self.Widget`) false false)
    (else
      (`PrimitiveComponent.SetRenderCustomDepth` _staticmesh false)
      (`PrimitiveComponent.SetCustomDepthStencilValue` _staticmesh 0)
      (`SceneComponent.SetHiddenInGame` (`self.Widget`) true false)))
  ;[1 1 1 0.5] Set or Update Item in focus widget
  (`/Engine/EditorBlueprintResources/StandardMacros.IsValid` _widget_focusinteraction
    (:`Is Valid`
      (`/Game/InventorySystem_0_4/Blueprints/UserInterfaces/Game/Item/WBP_FocusItem.Set_Item` _widget_focusinteraction (`self.Item`)))
    (:`Is Not Valid`
      (bind _aswbp_focus_item (cast `/Game/InventorySystem_0_4/Blueprints/UserInterfaces/Game/Item/WBP_FocusItem` (`WidgetComponent.GetWidget` (`self.Widget`))))
      (bind _output_get (set `self.Widget_FocusInteraction` _aswbp_focus_item))
      (`/Game/InventorySystem_0_4/Blueprints/UserInterfaces/Game/Item/WBP_FocusItem.Set_Item` _output_get (`self.Item`)))))

(fn `UserConstructionScript`
  (bind (_datatable _rowname) (break `DataTableRowHandle` (`.Item_2_7B2F9D1C44664DE095F72AA76ADB4E1C` (break `/Game/InventorySystem_0_4/Blueprints/Structures/F_Item` (`self.Item`)))))
  (bind _returnvalue (`|GetDataTableRow` _datatable _rowname)
    (:`then`
      (`StaticMeshComponent.SetStaticMesh` (`self.StaticMesh`) (`.StaticMesh_20_D34A863A40279183967777A1310ABFB5` (break `/Game/InventorySystem_0_4/Blueprints/Structures/F_ItemData` _returnvalue))))))