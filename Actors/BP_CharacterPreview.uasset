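; Character preview actor that renders a modular character, with its equipment and outfit meshes, into a render target through a scene capture.
; On BeginPlay it creates the render target, feeds it into a dynamic M_CharacterPreview material, and hides the sky sphere from the capture.
; Gear meshes follow the body via leader pose.
; An event swaps meshes by equipment or outfit type, while SetupAllMesh syncs every slot with the main character.
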(event `self.ReceiveBeginPlay`
  ;[1 1 1 0.5] Setup
  (`self.Setup`))

(event `Add Mesh To Character Preview`
  (params (EquipmentType :type "/Game/InventorySystem_0_4/Blueprints/Enumerations/E_EquipmentSlotType Enum" :default "NewEnumerator3") (OutfitType :type "/Game/InventorySystem_0_4/Blueprints/Enumerations/E_OutfitSlotType Enum" :default "NewEnumerator0") (SkeletalMesh :type "SkeletalMesh Object Reference"))
  ;[1 1 1 0.5] Add Mesh To Character Preview
  (`SkinnedMeshComponent.SetSkinnedAssetAndUpdate` (select `/Game/InventorySystem_0_4/Blueprints/Enumerations/E_EquipmentSlotType` EquipmentType :`NewEnumerator3` (`self.Empty`) :`NewEnumerator0` (`self.Helmet`) :`NewEnumerator1` (`self.Armor`) :`NewEnumerator2` (`self.Backpack`) :!type "SkinnedMeshComponent Object Reference") SkeletalMesh true)
  (`SkinnedMeshComponent.SetSkinnedAssetAndUpdate` (select `/Game/InventorySystem_0_4/Blueprints/Enumerations/E_OutfitSlotType` OutfitType :`NewEnumerator0` (`self.Empty`) :`NewEnumerator1` (`self.Glasses`) :`NewEnumerator2` (`self.Tshirt`) :`NewEnumerator3` (`self.Gloves`) :`NewEnumerator4` (`self.Pants`) :`NewEnumerator5` (`self.Shoes`) :!type "SkinnedMeshComponent Object Reference") SkeletalMesh true))

(fn `Setup`
  (bind _returnvalue (`KismetRenderingLibrary.CreateRenderTarget2D` 2048 1024 "RTF_RGBA16f" (make `LinearColor` 0.0)))
  (bind _returnvalue_2 (`KismetMaterialLibrary.CreateDynamicMaterialInstance` "/Game/InventorySystem_0_4/Materials/M_CharacterPreview.M_CharacterPreview"))
  (`MaterialInstanceDynamic.SetTextureParameterValue` _returnvalue_2 "Final Color" _returnvalue)
  (set `self.MaterialInstance` _returnvalue_2)
  (set `SceneCaptureComponent2D.TextureTarget` _returnvalue (`self.SceneCaptureComponent2D`))
  (bind _outactors (`GameplayStatics.GetAllActorsOfClass` "/Engine/EngineSky/BP_Sky_Sphere.BP_Sky_Sphere_C"))
  (bind _output (`|GetArrayItem` _outactors))
  (`/Engine/EditorBlueprintResources/StandardMacros.IsValid` _output
    (:`Is Valid`
      (`SceneCaptureComponent.HideActorComponents` (`self.SceneCaptureComponent2D`) _output false))))

(fn `Setup_AllMesh`
  (params (Helmet :type "SkinnedAsset Object Reference") (Tshirt :type "SkinnedAsset Object Reference") (Armor :type "SkinnedAsset Object Reference") (Backpack :type "SkinnedAsset Object Reference") (Pants :type "SkinnedAsset Object Reference") (Shoes :type "SkinnedAsset Object Reference") (Glasses :type "SkinnedAsset Object Reference") (Gloves :type "SkinnedAsset Object Reference"))
  ;[1 1 1 0.5] This function synchronizes the meshes between the Main Character and the Character Preview to make development easier.
  (`SkinnedMeshComponent.SetSkinnedAssetAndUpdate` (`self.Helmet`) Helmet true)
  (`SkinnedMeshComponent.SetSkinnedAssetAndUpdate` (`self.Tshirt`) Tshirt true)
  (`SkinnedMeshComponent.SetSkinnedAssetAndUpdate` (`self.Armor`) Armor true)
  (`SkinnedMeshComponent.SetSkinnedAssetAndUpdate` (`self.Backpack`) Backpack true)
  (`SkinnedMeshComponent.SetSkinnedAssetAndUpdate` (`self.Pants`) Pants true)
  (`SkinnedMeshComponent.SetSkinnedAssetAndUpdate` (`self.Shoes`) Shoes true)
  (`SkinnedMeshComponent.SetSkinnedAssetAndUpdate` (`self.Glasses`) Glasses true)
  (`SkinnedMeshComponent.SetSkinnedAssetAndUpdate` (`self.Gloves`) Gloves true))

(fn `UserConstructionScript`
  (`SkinnedMeshComponent.SetLeaderPoseComponent` (`self.Shoes`) (`self.SkeletalMesh`) false false)
  (`SkinnedMeshComponent.SetLeaderPoseComponent` (`self.Tshirt`) (`self.SkeletalMesh`) false false)
  (`SkinnedMeshComponent.SetLeaderPoseComponent` (`self.Glasses`) (`self.SkeletalMesh`) false false)
  (`SkinnedMeshComponent.SetLeaderPoseComponent` (`self.Pants`) (`self.SkeletalMesh`) false false)
  (`SkinnedMeshComponent.SetLeaderPoseComponent` (`self.Armor`) (`self.SkeletalMesh`) false false)
  (`SkinnedMeshComponent.SetLeaderPoseComponent` (`self.Gloves`) (`self.SkeletalMesh`) false false)
  (`SkinnedMeshComponent.SetLeaderPoseComponent` (`self.Backpack`) (`self.SkeletalMesh`) false false)
  (`SkinnedMeshComponent.SetLeaderPoseComponent` (`self.Helmet`) (`self.SkeletalMesh`) false false))